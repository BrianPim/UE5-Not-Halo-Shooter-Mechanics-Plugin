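; Ranged weapon Blueprint that spawns a projectile toward the player's aim point whenever the weapon is used.
; A camera trace finds the aim point and orients the muzzle-socket spawn toward it, falling back to the socket transform on a miss.
; The projectile receives the player as owner and instigator, and their primary weapon as parent.
; The player reference is cached on BeginPlay and retried on use to handle an initialization race.
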(event `self.ReceiveBeginPlay`
  (add `self.OnWeaponUsed` (delegate `OnWeaponUsed_Event`))
  (`self.TryAssignPlayerAndWeapon`))

(event `OnWeaponUsed_Event`
  (bind _playercharacter (`self.PlayerCharacter`))
  ;[1 1 1] Assigning Player & Weapon is race condition-y on BeginPlay, so we check here as well to make sure values have been cached correctly.
  (if (== (`self.PlayerCharacter`) null)
    (`self.TryAssignPlayerAndWeapon`))
  ;[1 1 1] Custom OnWeaponUsed Functionality. Casts a ray from the projectile spawn point to where the player is aiming in order to  provide the projectile with an accurate transform.
  (bind _projectiletransform (`self.CalculateProjectileTransform`))
  (bind _returnvalue (`|SpawnActorFromClass` (`self.ProjectileToSpawn`) _projectiletransform "AlwaysSpawn" "MultiplyWithRoot" _playercharacter _playercharacter))
  (`NotHaloProjectile.SetParentWeapon` _returnvalue (`NotHaloPlayerCharacter.GetPrimaryWeapon` _playercharacter)))

(fn `CalculateProjectileTransform`
  (returns (ProjectileTransform :type "Transform Structure"))
  (bind _weaponmesh (`self.WeaponMesh`))
  (bind _playercharacter (`self.PlayerCharacter`))
  (bind _spawnsocketname (`self.SpawnSocketName`))
  (bind _returnvalue (`SceneComponent.GetSocketLocation` _weaponmesh _spawnsocketname))
  (bind _firstpersoncamera (`NotHaloPlayerCharacter.FirstPersonCamera` _playercharacter))
  (bind _returnvalue_2 (`SceneComponent.K2_GetComponentLocation` _firstpersoncamera))
  (bind (_outhit _returnvalue_3) (`KismetSystemLibrary.LineTraceSingle` _returnvalue_2 (+ _returnvalue_2 (* (`SceneComponent.GetForwardVector` _firstpersoncamera) 50000.0)) "TraceTypeQuery2" false (`|MakeArray` _playercharacter (`NotHaloPlayerCharacter.GetPrimaryWeapon` _playercharacter) :!type "Actor Object Reference") "ForDuration"))
  (if _returnvalue_3
    (return (`KismetMathLibrary.MakeTransform` _returnvalue (`KismetMathLibrary.FindLookAtRotation` _returnvalue (`.Location` (`GameplayStatics.BreakHitResult` _outhit)))))
    (else
      (return (`SceneComponent.GetSocketTransform` _weaponmesh _spawnsocketname "RTS_World")))))

(fn `TryAssignPlayerAndWeapon`
  (bind _returnvalue (`self.GetWeaponHolderPawn`))
  (if (!= _returnvalue null)
    (bind _asbp_not_halo_player_character (cast `/NotHaloShooterMechanics/Core/Player/BP_NotHaloPlayerCharacter` _returnvalue))
    (set `self.PlayerCharacter` _asbp_not_halo_player_character)))

(fn `UserConstructionScript`)