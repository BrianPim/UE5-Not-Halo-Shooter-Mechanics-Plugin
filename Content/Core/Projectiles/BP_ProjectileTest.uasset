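; Test projectile actor that damages the player character it hits, draining shield before health.
; When the ProjectileMovementComponent stops, it casts the hit actor to NotHaloPlayerCharacter and skips damage on its instigator.
; Damage goes to shield if any remains, otherwise to health.
; It destroys itself after health damage or non-player hits, but not after instigator hits or shield hits, since the follow-up check reads the cached pre-hit shield value.
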(event `self.ProjectileMovementComponent.OnProjectileStop`
  (params (ImpactResult :type "HitResult Structure (by ref)"))
  (bind _damage (`self.Damage`))
  (bind _hitplayer (`self.HitPlayer`))
  (bind _asnot_halo_player_character (cast `NotHaloPlayerCharacter` (`.HitActor` (`GameplayStatics.BreakHitResult` ImpactResult)))
    (:`then`
      (`/Engine/EditorBlueprintResources/StandardMacros.IsValid` _asnot_halo_player_character
        (:`Is Valid`
          (set `self.HitPlayer` _asnot_halo_player_character)
          (if (!= _asnot_halo_player_character (`self.GetInstigator`))
            (set `self.HitPlayerShield` (`NotHaloPlayerCharacter.GetShield` _hitplayer))
            (set `self.HitPlayerHealth` (`NotHaloPlayerCharacter.GetHealth` _hitplayer))
            (if (> (`self.HitPlayerShield`) 0)
              (`NotHaloPlayerCharacter.UpdateShield` (`self.HitPlayer`) (- (`self.HitPlayerShield`) _damage))
              (if (<= (`self.HitPlayerShield`) 0)
                (`NotHaloPlayerCharacter.UpdateHealth` (`self.HitPlayer`) (- (`self.HitPlayerHealth`) _damage) :!label _label)
                (`self.K2_DestroyActor`))
              (else
                (goto _label)))))
        (:`Is Not Valid`
          (`self.K2_DestroyActor` :!label _label_2))))
    (:`CastFailed`
      (goto _label_2))))

(fn `UserConstructionScript`)