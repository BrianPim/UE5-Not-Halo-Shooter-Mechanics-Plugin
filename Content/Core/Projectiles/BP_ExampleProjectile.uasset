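; Example projectile actor that damages or headshot-kills NotHalo player characters when its projectile movement stops.
; Hitting the instigator only sets mutual move-ignore; other players take damage and the projectile destroys itself, as it does on non-player hits.
; A headshot requires the holder's primary weapon to allow it, a head-bone hit and depleted shields, then kills and applies an impulse at that bone.
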(event `self.ProjectileMovementComponent.OnProjectileStop`
  (params (ImpactResult :type "HitResult Structure (by ref)"))
  (bind (_bblockinghit _binitialoverlap _time _distance _location _impactpoint _normal _impactnormal _physmat _hitactor _hitcomponent _hitbonename) (`GameplayStatics.BreakHitResult` ImpactResult))
  (bind _returnvalue (`self.GetInstigator`))
  (bind _hitplayer (`self.HitPlayer`))
  (bind _hitbonename_2 (`self.HitBoneName`))
  (bind _mesh (`Character.Mesh` _hitplayer))
  (bind _returnvalue_location (`KismetMathLibrary.BreakTransform` (`SkinnedMeshComponent.GetBoneTransform` _mesh _hitbonename_2 "RTS_World")))
  ;[1 1 1] Try to get a player on projectile hit.
  (bind _asnot_halo_player_character (cast `NotHaloPlayerCharacter` _hitactor)
    (:`then`
      (`/Engine/EditorBlueprintResources/StandardMacros.IsValid` _asnot_halo_player_character
        (:`Is Valid`
          (bind _output_get (set `self.HitPlayer` _asnot_halo_player_character))
          (set `self.HitBoneName` _hitbonename)
          ;[1 1 1] Check if player is NOT the one who spawned the projectile. If true, do damage and destroy the projectile. If false, ignore.
          (if (!= _output_get _returnvalue)
            (bind _asnot_halo_player_character_2 (cast `NotHaloPlayerCharacter` _returnvalue))
            (bind _headshotallowed (`self.CheckHeadshotAllowed`))
            (if _headshotallowed
              (`NotHaloPlayerCharacter.Kill` _hitplayer _asnot_halo_player_character_2)
              (`PrimitiveComponent.AddImpulseAtLocation` _mesh (* (`KismetMathLibrary.Normal` (- _returnvalue_location (`SceneComponent.K2_GetComponentLocation` (`self.ProjectileMesh`)))) (`self.HitImpulseForce`)) _returnvalue_location _hitbonename_2)
              (else
                (`NotHaloPlayerCharacter.NotHaloApplyDamage` _hitplayer _asnot_halo_player_character_2 (`self.Damage`))))
            (`self.K2_DestroyActor`)
            (else
              (`PrimitiveComponent.IgnoreActorWhenMoving` (`self.ProjectileMesh`) _hitplayer true)
              (`PrimitiveComponent.IgnoreActorWhenMoving` (`Character.CapsuleComponent` _hitplayer) self true))))))
    (:`CastFailed`
      (`self.K2_DestroyActor`))))

(fn `CheckHeadshotAllowed`
  (returns (HeadshotAllowed :type Boolean))
  (bind _hitplayer (`self.HitPlayer`))
  (bind _asnot_halo_player_character (cast `NotHaloPlayerCharacter` (`NotHaloWeaponBase.GetWeaponHolderPawn` (`self.ParentWeapon`))))
  (return (and (`NotHaloWeaponBase.HeadshotsAllowed` (`NotHaloPlayerCharacter.GetPrimaryWeapon` _asnot_halo_player_character)) (== (`self.HitBoneName`) (`NotHaloPlayerCharacter.HeadshotBoneName` _hitplayer)) (<= (`NotHaloPlayerCharacter.GetShield` _hitplayer) 0))))

(fn `TryHitPlayer`
  (params (HitResult :type "HitResult Structure"))
  (returns (HitPlayer :type "NotHaloPlayerCharacter Object Reference"))
  (bind _asnot_halo_player_character (cast `NotHaloPlayerCharacter` (`.HitActor` (`GameplayStatics.BreakHitResult` HitResult))))
  (return _asnot_halo_player_character))

(fn `UserConstructionScript`)